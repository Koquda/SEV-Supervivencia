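; Weapon actor Blueprint that fires projectiles and launches grenades from the transform of its Arrow component.
; Shoot uses a DoOnce reset after a short delay to limit fire rate, spawning a projectile, brief sparks and a laser sound.
; After the sparks are removed, it decrements Ammo on the Jugador actor found in the world.
; ShootGranade spawns a scaled-down grenade and sets its physics velocity along the Arrow's forward vector.
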(event `Shoot`
  (bind _returnvalue (`SceneComponent.K2_GetComponentToWorld` (`self.Arrow`)))
  (`/Engine/EditorBlueprintResources/StandardMacros.DoOnce` false :!label _label
    (:`Completed`
      (`|ExecutionSequence`
        (:`then_0`
          (`|SpawnActorFromClass` "/Game/BP_Projectile.BP_Projectile_C" _returnvalue "Undefined" "OverrideRootScale" null null)
          (bind _returnvalue_2 (`GameplayStatics.SpawnEmitterAtLocation` "/Game/StarterContent/Particles/P_Sparks.P_Sparks" (.location _returnvalue)))
          (`KismetSystemLibrary.Delay` 0.2)
          (`ActorComponent.K2_DestroyComponent` _returnvalue_2)
          (bind _returnvalue_3 (`GameplayStatics.GetActorOfClass` "/Game/Player/Jugador.Jugador_C"))
          ;[0.2746 1 0.3358] Ampliacion 3
          (set `/Game/Player/Jugador.Ammo` (- (`/Game/Player/Jugador.Ammo` _returnvalue_3) 1) _returnvalue_3))
        (:`then_1`
          (`KismetSystemLibrary.Delay` 0.5)
          (goto _label :!via `Reset`))
        (:`then_2`
          (`GameplayStatics.PlaySoundAtLocation` "/Game/Sonidos/laser2.laser2" (`self.K2_GetActorLocation`) (struct) 1.0 1.0 0.0 null null null))))))

(event `ShootGranade`
  (bind _rotation (.rotation (`SceneComponent.K2_GetComponentToWorld` (`self.Arrow`))))
  ;[0.02078 0.9901 1] Ampliacion 5
  (bind _returnvalue (`|SpawnActorFromClass` "/Game/Granades/BP_Granade.BP_Granade_C" (`KismetMathLibrary.MakeTransform` (.location (`SceneComponent.K2_GetComponentToWorld` (`self.Arrow`))) _rotation (0.2 0.2 0.2)) "Undefined" "OverrideRootScale" null null))
  (`PrimitiveComponent.SetPhysicsLinearVelocity` (`/Game/Granades/BP_Granade.StaticMesh` _returnvalue) (* (`KismetMathLibrary.GetForwardVector` _rotation) 1000.0) false "None"))

(fn `UserConstructionScript`)