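; BP_Enemy is an enemy that chases the player using AI movement.
; On BeginPlay it finds and caches the Jugador actor, then starts FollowPlayer after a short delay.
; FollowPlayer checks that the reference is valid, runs AI MoveTo toward it, and calls itself again only on success, so a failed move ends the chase.
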(event `FollowPlayer`
  (bind _jugador (`self.Jugador`)
    (:`then`
      (`|AIMoveTo` self (0.0 0.0 0.0) _jugador 50.0
        (:`OnSuccess`
          (`self.FollowPlayer`))))
    (:`else`)))

(event `self.ReceiveBeginPlay`
  (bind _returnvalue (`GameplayStatics.GetActorOfClass` "/Game/Jugador.Jugador_C"))
  (set `self.Jugador` _returnvalue)
  (`KismetSystemLibrary.Delay` 0.1)
  (`self.FollowPlayer`))

(fn `UserConstructionScript`
  (`parent.UserConstructionScript`))